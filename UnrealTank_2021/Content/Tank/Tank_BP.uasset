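; Tank Blueprint that handles player camera aiming for the third-person view.
; AimVertical pitches HorizontalGimbal and AimHorizontal yaws SpringArm3rdP, splitting the axes across two components, with input scaled by frame delta time.
; SwitchCameraView is unfinished: it only calls a local rotation on SpringArmFP with no delta set.
; The default events and construction script are empty.
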(event `InputAxis|AimVertical`
  (params (AxisValue :type "Float (single-precision)"))
  ;[1 1 1] 3rd Person Camera Input Binding
  (`SceneComponent.K2_AddLocalRotation` (`self.HorizontalGimbal`) (`KismetMathLibrary.MakeRotator` 0.0 (* AxisValue (`GameplayStatics.GetWorldDeltaSeconds`) 10.0)) false false))

(event `InputAxis|AimHorizontal`
  (params (AxisValue :type "Float (single-precision)"))
  ;[1 1 1] 3rd Person Camera Input Binding
  (`SceneComponent.K2_AddLocalRotation` (`self.SpringArm_3rdP`) (`KismetMathLibrary.MakeRotator` 0.0 0.0 (* AxisValue (`GameplayStatics.GetWorldDeltaSeconds`) 10.0)) false false))

(event `InputAction|SwitchCameraView`
  (params (Key :type "Key Structure"))
  ;[1 1 1] Control both cameras
  (:`Pressed`
    (`SceneComponent.K2_AddLocalRotation` (`self.SpringArm_FP`) (`KismetMathLibrary.MakeRotator` 0.0) false false)))

(fn `UserConstructionScript`)